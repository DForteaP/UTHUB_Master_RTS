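; Base AI controller that receives generic unit orders, each carrying an action, location, target actor and ID.
; GiveGenericOrder handles only one action type, running the move AI component's action once that component validates the order.
; GetAllModules lazily caches the controller's AI module components in a map keyed by action, though the order event does not use it.
; GetUnitRef is an empty stub.
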(event EventGiveGenericOrder
  (params (Action :type E_Actions%20Enum :default "NewEnumerator0") (Location :type Vector :default "0, 0, 0") (Actor :type Actor%20Object%20Reference) (Id :type Name :default "None"))
  (bind _ac_moveai (Variables|Default|GetAC_MoveAI))
  (if (Utilities|Enum|Equal(Enum) Action "NewEnumerator11")
    (bind _yes (Default|IsValidforOrder _ac_moveai Location Actor Id))
    (if _yes
      (Default|DoAction _ac_moveai))))

(fn ConstructionScript)

(fn GetUnitRef)

(fn GetAllModules
  (if (Utilities|Map|IsEmpty (Variables|Default|GetListModules))
    (bind _output_get (LocalVariables|SetAICList (Actor|GetComponentsByClass "/Game/Blueprints/Components/AC_ModuleAIBase.AC_ModuleAIBase_C")))
    (for _array_element _output_get
      (Utilities|Map|Add (Variables|Default|GetListModules) (Variables|/Game/Blueprints/Components/AC_ModuleAIBase.AC_ModuleAIBase_C|GetAction _array_element) _array_element))
    (return (Variables|Default|GetListModules))
    (else
      (return (Variables|Default|GetListModules)))))