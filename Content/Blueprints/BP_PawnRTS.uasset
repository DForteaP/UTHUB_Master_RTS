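; RTS player pawn that handles camera panning and height-based zoom, click selection of a single actor, and map pings.
; Left-click traces select or deselect the actor through message calls and server/multicast-named events, refreshing the HUD with the selection.
; Right-click, number keys and the HUD ping board trace under the mouse to spawn a player-specific BP_FeedbackCursor.
; Orders to the selected actor are stubbed at a floor-tag check.
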(event Custom|SpawnRightCursor
  (params (Spawn%20Transform%20Location :type Vector) (Data%20Player :type S%20Data%20Player%20Structure) (Type :type E_TypePing%20Enum :default "NewEnumerator0"))
  (Game|SpawnActorfromClass "/Game/Blueprints/BP_FeedbackCursor.BP_FeedbackCursor_C" (Math|Transform|MakeTransform Spawn%20Transform%20Location "0, 0, 0" "1.000000,1.000000,1.000000") "Undefined" "MultiplyWithRoot" 0 Data%20Player Type 0))

(event Custom|SelectElementOnServer
  (params (Target :type Object%20Object%20Reference))
  (CallFunction|SelectElementsMulti Target (Variables|/Game/Blueprints/PC_RTS.PC_RTS_C|GetDataPlayer (CallFunction|GetPCRef))))

(event Custom|ShowRightCursor
  (params (CurrentTypePing :type E_TypePing%20Enum :default "NewEnumerator0"))
  (bind _pc_rts (CallFunction|GetPCRef))
  (bind (_worldlocation _worlddirection) (Game|Player|ConvertMouseLocationToWorldSpace _pc_rts))
  (Variables|Default|SetCurrentTypePing CurrentTypePing)
  (bind _output_get (Variables|Default|SetInitialLocationClick _worldlocation))
  (bind (_outhit _returnvalue) (Collision|LineTraceByChannel _output_get (+ _worldlocation (* _worlddirection 1e+06)) "TraceTypeQuery1" false 0 "None"))
  (if _returnvalue
    (CallFunction|SpawnRightCursorMulti (.ImpactPoint (Collision|BreakHitResult _outhit)))
    (CallFunction|GiveOrdertoSelectedActor (.ImpactPoint (Collision|BreakHitResult _outhit)) (.HitActor (Collision|BreakHitResult _outhit)))))

(event Custom|SelectElementsMulti
  (params (Target :type Object%20Object%20Reference) (Data%20Player :type S%20Data%20Player%20Structure))
  (bind _pc_rts (CallFunction|GetPCRef))
  (bind _hud_rts (Default|GetHUDRef _pc_rts))
  (bind _data (Class|BPISelectable|Select(Message) Target (.Color (Utilities|Struct|BreakS_DataPlayer Data%20Player)) (CallFunction|GetPCRef)))
  (Utilities|IsValid _pc_rts
    (:Is%20Valid
      (Utilities|IsValid _hud_rts
        (:Is%20Valid
          (Default|RefreshInfoItemSelected _hud_rts _data Target))))))

(event Custom|RemoveSelectDecalOnServer
  (params (Target :type Object%20Object%20Reference))
  (CallFunction|RemoveElementMulti Target))

(event Custom|RemoveElementMulti
  (params (Target :type Object%20Object%20Reference))
  (Class|BPISelectable|DeSelect(Message) Target (CallFunction|GetPCRef)))

(event Custom|SetNewPingType
  (params (CurrentTypePing :type E_TypePing%20Enum :default "NewEnumerator0"))
  ;[0.3347 0.1329 1] PINGS
  (bind _output_get (Variables|Default|SetCurrentTypePing CurrentTypePing))
  (CallFunction|ShowRightCursor _output_get))

(event Custom|ShowPing
  (params (TypePing :type E_TypePing%20Enum :default "NewEnumerator0"))
  ;[0.3347 0.1329 1] PINGS
  (CallFunction|SetNewPingType TypePing))

(event Custom|SpawnRightCursorMulti
  (params (Spawn%20Transform%20Location :type Vector))
  (CallFunction|SpawnRightCursor Spawn%20Transform%20Location (Variables|/Game/Blueprints/PC_RTS.PC_RTS_C|GetDataPlayer (CallFunction|GetPCRef)) (Variables|Default|GetCurrentTypePing)))

(event Input|EnhancedActionEvents|EnhancedInputActionIA_Zoom
  (params (ActionValue :type Float%20%28double-precision%29) (ElapsedSeconds :type Float%20%28double-precision%29) (TriggeredSeconds :type Float%20%28double-precision%29) (InputAction :type Input%20Action%20Object%20Reference :default "/Game/Inputs/IA_Zoom.IA_Zoom"))
  (bind _camera (Variables|Default|GetCamera))
  (bind _returnvalue (Transformation|GetWorldLocation _camera))
  ;[1 0.4754 0.5353] Zoom
  (Variables|Default|SetZoomAmount (Math|Float|Clamp(Float) (+ (Variables|Default|GetZoomAmount) (* ActionValue 7.0)) -2e+02 4e+02))
  (Transformation|SetWorldLocation _camera (Math|Vector|MakeVector (.x _returnvalue) (.y _returnvalue) (+ (.z (Variables|Default|GetLocationCamera)) (Variables|Default|GetZoomAmount))) false true))

(event Input|EnhancedActionEvents|EnhancedInputActionIA_4
  (params (ActionValue :type Boolean) (ElapsedSeconds :type Float%20%28double-precision%29) (TriggeredSeconds :type Float%20%28double-precision%29) (InputAction :type Input%20Action%20Object%20Reference :default "/Game/Inputs/IA_4.IA_4"))
  ;[0.3347 0.1329 1] PINGS
  (:Started
    (CallFunction|SetNewPingType "NewEnumerator3")))

(event Input|EnhancedActionEvents|EnhancedInputActionIA_Movement
  (params (ActionValue :type Vector%202D%20Structure) (ElapsedSeconds :type Float%20%28double-precision%29) (TriggeredSeconds :type Float%20%28double-precision%29) (InputAction :type Input%20Action%20Object%20Reference :default "/Game/Inputs/IA_Movement.IA_Movement"))
  (Class|PawnMovementComponent|AddInputVector (Variables|Default|GetFloatingPawnMovement) (Math|Conversions|ToVector(Vector2D) ActionValue) false))

(event Input|EnhancedActionEvents|EnhancedInputActionIA_Left
  (params (ActionValue :type Boolean) (ElapsedSeconds :type Float%20%28double-precision%29) (TriggeredSeconds :type Float%20%28double-precision%29) (InputAction :type Input%20Action%20Object%20Reference :default "/Game/Inputs/IA_Left.IA_Left"))
  (bind _pc_rts (CallFunction|GetPCRef))
  (bind (_worldlocation _worlddirection) (Game|Player|ConvertMouseLocationToWorldSpace _pc_rts))
  (:Started
    (bind (_outhit _returnvalue) (Collision|LineTraceByChannel _worldlocation (+ _worldlocation (* _worlddirection 1e+06)) "TraceTypeQuery3" false 0 "None"))
    (if _returnvalue
      (bind _selectedactor (Variables|Default|GetSelectedActor)
        (:then
          (Class|BPISelectable|DeSelect(Message) _selectedactor)
          (CallFunction|RemoveSelectDecalonServer _selectedactor)
          (Variables|Default|SetSelectedActor 0))
        (:else
          _))
      (CallFunction|SelectElementonServer (.HitActor (Collision|BreakHitResult _outhit)))
      (Variables|Default|SetSelectedActor (.HitActor (Collision|BreakHitResult _outhit)))
      (else
        (bind _selectedactor_2 (Variables|Default|GetSelectedActor)
          (:then
            (Class|BPISelectable|DeSelect(Message) _selectedactor_2)
            (CallFunction|RemoveSelectDecalonServer _selectedactor_2)
            (Variables|Default|SetSelectedActor 0))
          (:else))))))

(event Input|EnhancedActionEvents|EnhancedInputActionIA_Right
  (params (ActionValue :type Boolean) (ElapsedSeconds :type Float%20%28double-precision%29) (TriggeredSeconds :type Float%20%28double-precision%29) (InputAction :type Input%20Action%20Object%20Reference :default "/Game/Inputs/IA_Right.IA_Right"))
  (CallFunction|ShowRightCursor "NewEnumerator0"))

(event Input|EnhancedActionEvents|EnhancedInputActionIA_ShowPings
  (params (ActionValue :type Boolean) (ElapsedSeconds :type Float%20%28double-precision%29) (TriggeredSeconds :type Float%20%28double-precision%29) (InputAction :type Input%20Action%20Object%20Reference :default "/Game/Inputs/IA_ShowPings.IA_ShowPings"))
  ;[0.3347 0.1329 1] PINGS
  (:Started
    (Default|ShowMessagesBoard (Default|GetHUDRef (CallFunction|GetPCRef)) (delegate Custom|ShowPing)))
  (:Completed
    (CallFunction|ShowRightCursor "NewEnumerator0")
    (Default|ShowMessagesBoard (Default|GetHUDRef (CallFunction|GetPCRef)))))

(event Input|EnhancedActionEvents|EnhancedInputActionIA_1
  (params (ActionValue :type Boolean) (ElapsedSeconds :type Float%20%28double-precision%29) (TriggeredSeconds :type Float%20%28double-precision%29) (InputAction :type Input%20Action%20Object%20Reference :default "/Game/Inputs/IA_1.IA_1"))
  ;[0.3347 0.1329 1] PINGS
  (:Started
    (CallFunction|SetNewPingType "NewEnumerator0")))

(event Input|EnhancedActionEvents|EnhancedInputActionIA_2
  (params (ActionValue :type Boolean) (ElapsedSeconds :type Float%20%28double-precision%29) (TriggeredSeconds :type Float%20%28double-precision%29) (InputAction :type Input%20Action%20Object%20Reference :default "/Game/Inputs/IA_2.IA_2"))
  ;[0.3347 0.1329 1] PINGS
  (:Started
    (CallFunction|SetNewPingType "NewEnumerator1")))

(event Input|EnhancedActionEvents|EnhancedInputActionIA_3
  (params (ActionValue :type Boolean) (ElapsedSeconds :type Float%20%28double-precision%29) (TriggeredSeconds :type Float%20%28double-precision%29) (InputAction :type Input%20Action%20Object%20Reference :default "/Game/Inputs/IA_3.IA_3"))
  ;[0.3347 0.1329 1] PINGS
  (:Started
    (CallFunction|SetNewPingType "NewEnumerator2")))

(event EventBeginPlay
  (Variables|Default|SetLocationCamera (Transformation|GetWorldLocation (Variables|Default|GetCamera))))

(fn ConstructionScript)

(fn GetPCRef
  (Variables|Default|GetPC%20RTS
    (:then
      _)
    (:else
      (bind _aspc_rts (Utilities|Casting|CastToPC_RTS (Components|GetOwner)))
      (Variables|Default|SetPC%20RTS _aspc_rts)))
  (return (Variables|Default|GetPC%20RTS)))

(fn GetGMRef
  (Variables|Default|GetGM%20RTS
    (:then
      _)
    (:else
      (bind _asgm_rts (Utilities|Casting|CastToGM_RTS (Game|GetGameMode)))
      (Variables|Default|SetGM%20RTS _asgm_rts)))
  (return (Variables|Default|GetGM%20RTS)))

(fn GiveOrdertoSelectedActor
  (params (Location :type Vector) (Actor :type Actor%20Object%20Reference))
  (Variables|Default|GetSelectedActor
    (:then
      (if (Actor|ActorHasTag Actor "floor")
        _))
    (:else)))