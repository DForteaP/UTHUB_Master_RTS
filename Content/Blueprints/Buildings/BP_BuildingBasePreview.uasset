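; Placement preview for RTS buildings, built from a data-table ID and snapped to the grid under the player's cursor every tick.
; A dynamic material on the grid collision shows whether the spot is valid and the building is affordable.
; Validity comes from collision overlaps: water-dependent buildings need a water or floor overlap, others need none.
; The inherited grid collision scaling is extended to widen X and Y.
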(event OnComponentBeginOverlap(BuildingGridCollision)
  (params (OverlappedComponent :type Primitive%20Component%20Object%20Reference) (OtherActor :type Actor%20Object%20Reference) (OtherComp :type Primitive%20Component%20Object%20Reference) (OtherBodyIndex :type Integer) (bFromSweep :type Boolean) (SweepResult :type Hit%20Result%20Structure%20%28by%20ref%29)))

(event OnComponentEndOverlap(BuildingGridCollision)
  (params (OverlappedComponent :type Primitive%20Component%20Object%20Reference) (OtherActor :type Actor%20Object%20Reference) (OtherComp :type Primitive%20Component%20Object%20Reference) (OtherBodyIndex :type Integer)))

(event EventBeginPlay
  (CallFunction|BuildfromDT (Variables|Default|GetIDPreview))
  (bind _returnvalue (Rendering|Material|CreateDynamicMaterialInstance "/Game/Materials/M_BuildingPreview_M.M_BuildingPreview_M" "None" "None" :!class /Script/Engine.KismetMaterialLibrary))
  (bind _output_get (Variables|Default|SetGrid_MI _returnvalue))
  (Rendering|Material|SetMaterial (Variables|Default|GetBuildingGridCollision) 0 _output_get))

(event EventTick
  (params (DeltaSeconds :type Float%20%28single-precision%29))
  (bind _location (Default|GetCursorPosition (CallFunction|GetPCRTS) "TraceTypeQuery4"))
  (CallFunction|ClamptoGrid _location)
  (CallFunction|ChangeMaterialColor))

(fn ConstructionScript
  (|CallParentFunction))

(fn GetPCRTS
  (Variables|Default|GetPC%20RTS
    (:then
      _)
    (:else
      (bind _aspc_rts (Utilities|Casting|CastToPC_RTS (Game|GetPlayerController 0)))
      (Variables|Default|SetPC%20RTS _aspc_rts)))
  (return (Variables|Default|GetPC%20RTS)))

(fn CanIBuildHere?
  (if (.NeedWater? (Utilities|Struct|BreakS_Buildings (Variables|Default|GetBuildingData)))
    (return (not (and (Utilities|Array|IsEmpty (Collision|GetOverlappingActors (Variables|Default|GetBuildingGridCollision) "/Game/Blueprints/BP_Water.BP_Water_C" :!class /Script/Engine.PrimitiveComponent)) (Utilities|Array|IsEmpty (Collision|GetOverlappingActors (Variables|Default|GetBuildingGridCollision) "/Game/Blueprints/BP_Floor.BP_Floor_C" :!class /Script/Engine.PrimitiveComponent)))))
    (else
      (return (Utilities|Array|IsEmpty (Collision|GetOverlappingActors (Variables|Default|GetBuildingGridCollision) 0 :!class /Script/Engine.PrimitiveComponent))))))

(fn ChangeMaterialColor
  (Rendering|Material|SetScalarParameterValue (Variables|Default|GetGrid_MI) "Status" (select (and (CallFunction|CanIBuildHere?) (CallFunction|CanIPayIt?)) 0.0 1.0) :!class /Script/Engine.MaterialInstanceDynamic))

(fn IsWater?
  (return (Utilities|Array|IsEmpty (Collision|GetOverlappingActors (Variables|Default|GetBuildingGridCollision) "/Game/Blueprints/BP_Water.BP_Water_C" :!class /Script/Engine.PrimitiveComponent))))

(fn ScaleGridCollision
  (bind _buildinggridcollision (Variables|Default|GetBuildingGridCollision))
  (bind _returnvalue (Transformation|GetWorldScale _buildinggridcollision))
  (|CallParentFunction)
  (Transformation|SetWorldScale3D _buildinggridcollision (Math|Vector|MakeVector (* (.x _returnvalue) 5.0) (* (.y _returnvalue) 5.0) (.z _returnvalue))))