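; Base RTS building actor that configures itself from data tables by unit ID and snaps to a 100-unit grid.
; BeginPlay loads UI data, mesh, grid size and cost; the construction script scales grid collision and snaps location.
; Select adds a colored decal, tracks the selecting player and returns UI data flagging craftable units by unlocked investigations.
; Investigation and affordability checks query GS_RTS through a cached getter.
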(event EventDeSelect
  (params (PC :type PC%20RTS%20Object%20Reference))
  (bind _returnvalue (Actor|GetComponentbyClass "/Script/Engine.DecalComponent"))
  (Utilities|Array|RemoveItem (Variables|Default|GetSelectedByPlayers) PC)
  (Utilities|IsValid _returnvalue
    (:Is%20Valid
      (Components|DestroyComponent _returnvalue))))

(event EventBeginPlay
  (bind _idunit (Variables|Default|GetIDUnit))
  (bind _returnvalue (Utilities|GetDataTableRow "/Game/Blueprints/Structs/DT_ElementsUI.DT_ElementsUI" _idunit)
    (:then
      (Variables|Default|SetData _returnvalue)
      (CallFunction|BuildfromDT _idunit))))

(fn ConstructionScript
  (CallFunction|ScaleGridCollision)
  (CallFunction|CorrectPivotLocation)
  (CallFunction|ClamptoGrid (Transformation|GetActorLocation)))

(fn GetInfo
  (return (CallFunction|UpdateInvestigations (Variables|Default|GetData))))

(fn ClamptoGrid
  (params (InVec :type Vector))
  (bind (_x _y _z) (Math|Vector|BreakVector InVec))
  (Transformation|SetActorLocation (Math|Vector|MakeVector (Math|Conversions|ToFloat(Integer) (* (Math|Float|Round (/ _x 1e+02)) 100)) (Math|Conversions|ToFloat(Integer) (* (Math|Float|Round (/ _y 1e+02)) 100)) _z) false true))

(fn ScaleGridCollision
  (bind _buildingdata (Variables|Default|GetBuildingData))
  (bind _buildinggridcollision (Variables|Default|GetBuildingGridCollision))
  (bind _gridsize (Utilities|Struct|BreakS_Buildings _buildingdata))
  (bind (_x _y) (Math|Vector2D|BreakVector2D _gridsize))
  (Transformation|SetWorldScale3D _buildinggridcollision (Math|Vector|MakeVector _x _y (.z (Transformation|GetWorldScale _buildinggridcollision)))))

(fn CorrectPivotLocation
  (bind (_x _y) (Math|Vector2D|BreakVector2D))
  (Transformation|SetRelativeLocation (Variables|Default|GetBuildingGridCollision) (Math|Vector|MakeVector (* _x 5e+01) (* _y 5e+01) 0.0) false true))

(fn BuildfromDT
  (params (RowName :type Name))
  (bind _meshbuilding (Variables|Default|GetMeshBuilding))
  (Utilities|FlowControl|Sequence
    (:then_0
      (bind _returnvalue (Utilities|GetDataTableRow "/Game/Blueprints/Structs/DT_Buildings.DT_Buildings" RowName)
        (:then
          (Variables|Default|SetBuildingData _returnvalue)
          (CallFunction|ScaleGridCollision)
          (CallFunction|CorrectPivotLocation)
          (Components|StaticMesh|SetStaticMesh _meshbuilding (.StaticMesh (Utilities|Struct|BreakS_Buildings (Variables|Default|GetBuildingData))))
          (Transformation|SetRelativeTransform _meshbuilding (.Transform (Utilities|Struct|BreakS_Buildings (Variables|Default|GetBuildingData))) false true))))
    (:then_1
      (bind _returnvalue_2 (Utilities|GetDataTableRow "/Game/Blueprints/Structs/DT_Crafteable.DT_Crafteable" RowName)
        (:then
          (Variables|Default|SetCostCrafteables _returnvalue_2))))))

(fn GetPSRef
  (Variables|Default|GetPS%20RTS
    (:then
      _)
    (:else
      (bind _asps_rts (Utilities|Casting|CastToPS_RTS (Game|GetPlayerState 0)))
      (Variables|Default|SetPS%20RTS _asps_rts)))
  (return (Variables|Default|GetPS%20RTS)))

(fn CanIPayIt?
  (return (Default|CanIPayIt? (CallFunction|GetGSRef) (.Price (Utilities|Struct|BreakS_Crafteables (Variables|Default|GetCostCrafteables))))))

(fn GetGSRef
  (Variables|Default|GetGS%20RTS
    (:then
      _)
    (:else
      (bind _asgs_rts (Utilities|Casting|CastToGS_RTS (Game|GetGameState)))
      (Variables|Default|SetGS%20RTS _asgs_rts)))
  (return (Variables|Default|GetGS%20RTS)))

(fn UpdateInvestigations
  (params (DataBuilding :type S%20Data%20UI%20Structure))
  (bind _output_get (LocalVariables|SetInfoCraft DataBuilding))
  (bind _keys (Utilities|Map|Keys (.UnitsCrafteables (Utilities|Struct|BreakS_DataUI _output_get))))
  (for _array_element _keys
    (bind _allunlocked_ (CallFunction|CheckifIHaveInvestigation _array_element))
    (Utilities|Map|Add (.UnitsCrafteables (Utilities|Struct|BreakS_DataUI _output_get)) _array_element _allunlocked_))
  (return (LocalVariables|GetInfoCraft)))

(fn CheckifIHaveInvestigation
  (params (RowName :type Name))
  (bind _returnvalue (Utilities|GetDataTableRow "/Game/Blueprints/Structs/DT_Crafteable.DT_Crafteable" RowName)
    (:then
      (for _array_element (.InvestRequired (Utilities|Struct|BreakS_Crafteables _returnvalue))
        (bind _investunlocked_ (Default|InvestigationUnlocked? (CallFunction|GetGSRef) _array_element))
        (if (not _investunlocked_)
          (return false)))
      (return true))))

(fn IsAInvestigation?
  (params (RowName :type Name))
  (bind _returnvalue (Utilities|GetDataTableRow "/Game/Blueprints/Structs/DT_Crafteable.DT_Crafteable" RowName)
    (:then
      (return (Utilities|Enum|Equal(Enum) (.Type (Utilities|Struct|BreakS_Crafteables _returnvalue)) "NewEnumerator10")))))

(fn Select
  (params (Color :type Linear%20Color%20Structure) (PC :type PC%20RTS%20Object%20Reference))
  (bind _self self)
  (bind _scale (CallFunction|CalculateScaleDecal _self))
  (bind _returnvalue (AddComponent|AddDecalComponent false (Math|Transform|MakeTransform "0, 0, 0" "90.000000,0.000000,0.000000" (Math|Vector|MakeVector 1.0 (.y _scale) (.z _scale)))))
  (Rendering|Components|Decal|SetDecalMaterial _returnvalue "/Game/Materials/M_SelectedMaterial.M_SelectedMaterial")
  (bind _returnvalue_2 (Rendering|Material|CreateDynamicMaterialInstance "/Game/Materials/M_SelectedMaterial.M_SelectedMaterial" "None" "None" :!class /Script/Engine.KismetMaterialLibrary))
  (Rendering|Material|SetVectorParameterValue _returnvalue_2 "Color" Color :!class /Script/Engine.MaterialInstanceDynamic)
  (Rendering|Components|Decal|SetDecalMaterial _returnvalue _returnvalue_2)
  (Utilities|Array|AddUnique (Variables|Default|GetSelectedByPlayers) PC)
  (return (CallFunction|GetInfo)))