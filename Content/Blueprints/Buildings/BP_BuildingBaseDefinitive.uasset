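; Base building actor that configures itself from its DT_Buildings row, shows the owning player's name and color, and produces units or investigations.
; A capped construction pile works as a first-in, first-out queue, with a single timer crafting the front item.
; On completion, items with a valid class spawn as units at SpawnArea through the GS reference; others register as investigations by name.
; The next queued item then starts.
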(event Custom|CraftFirstObject
  (bind _output_get (Variables|Default|SetClassInfoToSpawn (Utilities|Array|Get(acopy) (Variables|Default|GetConstructPile))))
  (bind _returnvalue (Utilities|Time|SetTimerbyEvent (delegate Custom|SpawnCrafteable) (.Time (Utilities|Struct|BreakS_Crafteables _output_get))))
  (Variables|Default|SetTimerCraft _returnvalue))

(event Custom|AddElementToPile
  (params (Item :type S%20Crafteables%20Structure%20%28by%20ref%29))
  (if (CallFunction|IHaveSpaceinConstructPile?)
    (Utilities|Array|Add (Variables|Default|GetConstructPile) Item)
    (CallFunction|CheckifCraft)))

(event Custom|CheckIfCraft
  (if (not (Utilities|Time|IsValidTimerHandle (Variables|Default|GetTimerCraft)))
    (CallFunction|CraftFirstObject)))

(event Custom|SpawnCrafteable
  (bind _classinfotospawn (Variables|Default|GetClassInfoToSpawn))
  (bind (_price _name _icon _description _time _class) (Utilities|Struct|BreakS_Crafteables _classinfotospawn))
  (Utilities|Time|ClearandInvalidateTimerbyHandle (Variables|Default|GetTimerCraft))
  (if (Utilities|IsValidClass _class)
    (Default|SpawnUnitforPlayer (CallFunction|GetGSRef) _class (Transformation|GetWorldLocation (Variables|Default|GetSpawnArea)) (Components|GetOwner))
    (else
      (Default|AddInvestigation (CallFunction|GetGSRef) _name)))
  (Utilities|Array|RemoveIndex (Variables|Default|GetConstructPile))
  (if (not (Utilities|Array|IsEmpty (Variables|Default|GetConstructPile)))
    (CallFunction|CraftFirstObject)))

(event EventBeginPlay
  (bind _textrender (Variables|Default|GetTextRender))
  (bind _dataplayerowner (Variables|Default|GetDataPlayerOwner))
  (bind (_id _name _color) (Utilities|Struct|BreakS_DataPlayer _dataplayerowner))
  (|CallParentFunction)
  (bind _returnvalue (Utilities|GetDataTableRow "/Game/Blueprints/Structs/DT_Buildings.DT_Buildings" (Variables|Default|GetIDUnit))
    (:then
      (Variables|Default|SetBuildingData _returnvalue)
      (CallFunction|BuildfromDT (Variables|Default|GetIDUnit))
      (Rendering|SetVisibility (Variables|Default|GetBuildingGridCollision) false false)
      (Rendering|Components|TextRender|SetText _textrender (Utilities|Text|ToText(Name) _name))
      (Rendering|Components|TextRender|SetTextRenderColor _textrender (Math|Conversions|ToColor(LinearColor) _color)))))

(fn ConstructionScript
  (|CallParentFunction))

(fn IHaveSpaceinConstructPile?
  (return (< (Utilities|Array|Length (Variables|Default|GetConstructPile)) 4)))

(fn GetConstructPileInfo
  (return (Variables|Default|GetConstructPile) (Variables|Default|GetTimerCraft)))