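; BP_CharacterBase is a base unit character that can be selected and given orders, as in an RTS.
; On BeginPlay it loads its UI data from DT_ElementsUI by unit ID, and the authority spawns an AIC_Base and moves the unit toward Destiny.
; Selection adds a scaled, color-tinted decal and returns the unit data, while deselection destroys the decal.
; Orders pass through a server-named event to the cached AI controller.
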(event Custom|GiveGenericOrderServer
  (params (Action :type E_Actions%20Enum :default "NewEnumerator0") (Location :type Vector) (Actor :type Actor%20Object%20Reference) (Id :type Name))
  (Default|GiveGenericOrder (CallFunction|GetAIRef) Action Location Actor Id))

(event EventDeSelect
  (params (PC :type PC%20RTS%20Object%20Reference))
  (bind _returnvalue (Actor|GetComponentbyClass "/Script/Engine.DecalComponent"))
  (Utilities|IsValid _returnvalue
    (:Is%20Valid
      (Components|DestroyComponent _returnvalue))))

(event EventBeginPlay
  (Utilities|FlowControl|Sequence
    (:then_0
      (bind _returnvalue (Utilities|GetDataTableRow "/Game/Blueprints/Structs/DT_ElementsUI.DT_ElementsUI" (Variables|Default|GetIDUnit))
        (:then
          (Variables|Default|SetData _returnvalue))))
    (:then_1
      (Networking|SwitchHasAuthority
        (:Authority
          (bind _returnvalue_2 (Game|SpawnActorfromClass "/Game/Blueprints/AIC_Base.AIC_Base_C" (Math|Transform|MakeTransform "0, 0, 0" "0, 0, 0" "1.000000,1.000000,1.000000") "Undefined" "MultiplyWithRoot" 0 0))
          (Variables|Default|SetAIC%20Base _returnvalue_2)
          (AI|AIMoveTo self "0, 0, 0" (Variables|Default|GetDestiny) 5.0 false))))))

(event EventGiveGenericOrder
  (params (Action :type E_Actions%20Enum :default "NewEnumerator0") (Location :type Vector :default "0, 0, 0") (Actor :type Actor%20Object%20Reference) (Id :type Name :default "None"))
  (CallFunction|GiveGenericOrderServer Action Location Actor Id))

(fn ConstructionScript)

(fn GetInfo
  (return (Variables|Default|GetData)))

(fn GetAIRef
  (Variables|Default|GetAIC%20Base
    (:then
      _)
    (:else
      (bind _asaic_base (Utilities|Casting|CastToAIC_Base (AI|GetAIController self)))
      (Variables|Default|SetAIC%20Base _asaic_base)))
  (return (Variables|Default|GetAIC%20Base)))

(fn Select
  (params (Color :type Linear%20Color%20Structure) (PC :type PC%20RTS%20Object%20Reference))
  (bind _self self)
  (bind _scale (CallFunction|CalculateScaleDecal _self))
  (bind _returnvalue (AddComponent|AddDecalComponent false (Math|Transform|MakeTransform "0, 0, 0" "90.000000,0.000000,0.000000" (Math|Vector|MakeVector 1.0 (.y _scale) (.z _scale)))))
  (Rendering|Components|Decal|SetDecalMaterial _returnvalue "/Game/Materials/M_SelectedMaterial.M_SelectedMaterial")
  (bind _returnvalue_2 (Rendering|Material|CreateDynamicMaterialInstance "/Game/Materials/M_SelectedMaterial.M_SelectedMaterial" "None" "None" :!class /Script/Engine.KismetMaterialLibrary))
  (Rendering|Material|SetVectorParameterValue _returnvalue_2 "Color" Color :!class /Script/Engine.MaterialInstanceDynamic)
  (Rendering|Components|Decal|SetDecalMaterial _returnvalue _returnvalue_2)
  (return (CallFunction|GetInfo)))