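; BP_Cursor is an actor that shows a player's cursor in the world, labeled with that player's name and color.
; On BeginPlay it caches the W_CursorWorld from its widget component and initializes it from DataPlayer through SetData.
; Each Tick it eases toward DestinyLocation with VInterpTo and a teleporting move, skipping the update once it is within a small tolerance.
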(event EventTick
  (params (DeltaSeconds :type Float%20%28single-precision%29))
  (bind _returnvalue (Transformation|GetActorLocation))
  (if (not (Utilities|Operators|EqualEqual _returnvalue (Variables|Default|GetDestinyLocation) 0.2))
    (Transformation|SetActorLocation (Math|Interpolation|VInterpTo _returnvalue (Variables|Default|GetDestinyLocation) DeltaSeconds 2.0) false true)))

(event EventBeginPlay
  (bind _asw_cursor_world (Utilities|Casting|CastToW_CursorWorld (UserInterface|GetWidget (Variables|Default|GetWidget))))
  (Variables|Default|SetW%20Cursor%20World _asw_cursor_world)
  (CallFunction|SetData (Variables|Default|GetData%20Player)))

(fn ConstructionScript)

(fn SetData
  (params (DataPlayer :type S%20Data%20Player%20Structure))
  (bind (_id _name _color) (Utilities|Struct|BreakS_DataPlayer DataPlayer))
  (Default|Init (Variables|Default|GetW%20Cursor%20World) _name _color))