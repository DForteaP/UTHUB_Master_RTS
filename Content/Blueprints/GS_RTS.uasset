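; RTS Game State that holds a resource pool and researched investigations shared by all players, and spawns their buildings and units.
; A looping one-second timer gathers every player controller's cursor position and identity and sends the list back to each.
; Building spawns look up the actor in DT_Buildings, deduct the DT_Crafteable price and push updated resources to every player's UI.
; Helper functions check affordability and research unlocks.
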(event Custom|SyncPlayerCursor
  (bind _pcs (CallFunction|GetPCs))
  (Utilities|Array|Clear (Variables|Default|GetInfoCursors))
  (for _array_element _pcs
    (Utilities|Array|Add (Variables|Default|GetInfoCursors) (Utilities|Struct|MakeS_DataPlayer (.ID (Utilities|Struct|BreakS_DataPlayer (Variables|/Game/Blueprints/PC_RTS.PC_RTS_C|GetDataPlayer _array_element))) (.Name (Utilities|Struct|BreakS_DataPlayer (Variables|/Game/Blueprints/PC_RTS.PC_RTS_C|GetDataPlayer _array_element))) (.Color (Utilities|Struct|BreakS_DataPlayer (Variables|/Game/Blueprints/PC_RTS.PC_RTS_C|GetDataPlayer _array_element))) (Variables|/Game/Blueprints/PC_RTS.PC_RTS_C|GetCursorPosition _array_element))))
  (bind _pcs_2 (CallFunction|GetPCs))
  (for _array_element_2 _pcs_2
    (Default|ReceiveOtherCursors _array_element_2 (Variables|Default|GetInfoCursors))))

(event Custom|SpawnBuildForPlayer
  (params (PC :type PC%20RTS%20Object%20Reference) (Building :type Name) (Spawn%20Location :type Vector) (DataPlayerOwner :type S%20Data%20Player%20Structure))
  (bind _returnvalue (Utilities|GetDataTableRow "/Game/Blueprints/Structs/DT_Buildings.DT_Buildings" Building)
    (:then
      (CallFunction|AddRemoveResources (CallFunction|GetCost Building) false)
      (Game|SpawnActorfromClass (.Actor (Utilities|Struct|BreakS_Buildings _returnvalue)) (Math|Transform|MakeTransform Spawn%20Location "0, 0, 0" "1.000000,1.000000,1.000000") "Undefined" "MultiplyWithRoot" PC DataPlayerOwner 0 Building 0)
      (bind _pcs (CallFunction|GetPCs))
      (for _array_element _pcs
        (Default|UpdateResourcesUI _array_element (Variables|Default|GetResources))))))

(event Custom|SpawnUnitForPlayer
  (params (Class :type Actor%20Class%20Reference) (Spawn%20Transform%20Location :type Vector) (Owner :type Actor%20Object%20Reference) (Destiny :type Actor%20Object%20Reference))
  (bind _asbp_character_base (Utilities|Casting|CastToBP_CharacterBaseClass Class))
  (bind _output_get (Variables|Default|SetClass _asbp_character_base))
  (Game|SpawnActorfromClass _output_get (Math|Transform|MakeTransform Spawn%20Transform%20Location "0, 0, 0" "1.000000,1.000000,1.000000") "Undefined" "MultiplyWithRoot" Owner Destiny 0))

(event Custom|AddInvestigation
  (params (NewItem :type Text%20%28by%20ref%29))
  (CallFunction|AddInvestigations NewItem))

(event EventTick
  (params (DeltaSeconds :type Float%20%28single-precision%29)))

(event EventBeginPlay
  (Utilities|Time|SetTimerbyEvent (delegate Custom|SyncPlayerCursor) 1.0 true))

(fn ConstructionScript)

(fn GetPCs
  (if (== (Utilities|Array|Length (Variables|Default|GetPlayerArray)) (Utilities|Array|Length (Variables|Default|GetPCs)))
    (return (Variables|Default|GetPCs))
    (else
      (Utilities|Array|Clear (Variables|Default|GetPCs))
      (for _array_element (Variables|Default|GetPlayerArray)
        (bind _aspc_rts (Utilities|Casting|CastToPC_RTS (Game|GetPlayerController _array_element)))
        (Utilities|Array|Add (Variables|Default|GetPCs) _aspc_rts))
      (return (Variables|Default|GetPCs)))))

(fn AddRemoveResources
  (params (Resources :type Map%20of%20E_ResourceType%20Enums%20to%20Integers :default "NewEnumerator0") (Add? :type Boolean))
  (bind _keys (Utilities|Map|Keys Resources))
  (for _array_element _keys
    (for _array_element_2 (Variables|Default|GetResources)
      (if (Utilities|Enum|Equal(Enum) _array_element (.Resource (Utilities|Struct|BreakS_ResourceAmount _array_element_2)))
        (bind _resources (CallFunction|UpdateResource (.Resource (Utilities|Struct|BreakS_ResourceAmount _array_element_2)) (+ (.Amount (Utilities|Struct|BreakS_ResourceAmount _array_element_2)) (* (.Value (Utilities|Map|Find Resources _array_element)) (select Add? 1 -1)))))
        (Variables|Default|SetResources _resources))))
  (bind _pcs (CallFunction|GetPCs))
  (for _array_element_3 _pcs
    (Default|UpdateResourcesUI _array_element_3 (Variables|Default|GetResources))))

(fn MergeArraysIntoMap
  (params (Resource :type Array%20of%20E_ResourceType%20Enums :default "NewEnumerator0") (Amount :type Array%20of%20Integers))
  (Utilities|Array|Clear (LocalVariables|GetMap))
  (for (_array_element _array_index) Resource
    (Utilities|Array|Add (LocalVariables|GetMap) (Utilities|Struct|MakeS_ResourceAmount _array_element (Utilities|Array|Get(acopy) Amount _array_index))))
  (return (LocalVariables|GetMap)))

(fn SetResource
  (params (Resource :type E_ResourceType%20Enum :default "NewEnumerator0") (Amount :type Integer))
  (bind _resources (Variables|Default|GetResources))
  (for (_array_element _array_index) _resources
    (if (Utilities|Enum|Equal(Enum) (.Resource (Utilities|Struct|BreakS_ResourceAmount _array_element)) Resource)
      (Utilities|Array|SetArrayElem _resources _array_index (Utilities|Struct|MakeS_ResourceAmount (.Resource (Utilities|Struct|BreakS_ResourceAmount _array_element)) Amount) true))))

(fn CanIPayIt?
  (params (Costs :type Map%20of%20E_ResourceType%20Enums%20to%20Integers :default "NewEnumerator0"))
  (for _array_element (Variables|Default|GetResources)
    (if (not (>= (.Amount (Utilities|Struct|BreakS_ResourceAmount _array_element)) (.Value (Utilities|Map|Find Costs (.Resource (Utilities|Struct|BreakS_ResourceAmount _array_element))))))
      (if (not (Utilities|Enum|NotEqual(Enum) (.Resource (Utilities|Struct|BreakS_ResourceAmount _array_element)) "NewEnumerator3"))
        (return false))))
  (return true))

(fn UpdateResource
  (params (Resource :type E_ResourceType%20Enum :default "NewEnumerator0") (Amount :type Integer))
  (for (_array_element _array_index) (Variables|Default|GetResources)
    (if (Utilities|Enum|Equal(Enum) (.Resource (Utilities|Struct|BreakS_ResourceAmount _array_element)) Resource)
      (Utilities|Array|SetArrayElem (Variables|Default|GetResources) _array_index (Utilities|Struct|MakeS_ResourceAmount (.Resource (Utilities|Struct|BreakS_ResourceAmount _array_element)) Amount) true)
      (if (Utilities|Enum|Equal(Enum) (.Resource (Utilities|Struct|BreakS_ResourceAmount _array_element)) "NewEnumerator0")
        (Development|PrintText (Utilities|Text|FormatText "Ahora la madera es {x}" Amount)))))
  (return (Variables|Default|GetResources)))

(fn GetCost
  (params (Id :type Name))
  (bind _returnvalue (Utilities|GetDataTableRow "/Game/Blueprints/Structs/DT_Crafteable.DT_Crafteable" Id)
    (:then
      (return (.Price (Utilities|Struct|BreakS_Crafteables _returnvalue))))))

(fn InvestigationUnlocked?
  (params (ItemToFind :type Text%20%28by%20ref%29))
  (return (Utilities|Array|ContainsItem (Variables|Default|GetInvestigations) ItemToFind)))

(fn AddInvestigations
  (params (NewItem :type Text%20%28by%20ref%29))
  (Utilities|Array|AddUnique (Variables|Default|GetInvestigations) NewItem))