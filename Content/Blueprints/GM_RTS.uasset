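; GM_RTS is the RTS game mode that registers each joining player with a generated identity.
; On HandleStartingNewPlayer it casts the controller to PC_RTS and generates a GUID, a randomized "Fortea" name and a random color.
; The controller receives that data through AssignIDAndData and SetDataPlayer, and is stored in a Players map keyed by ID for GetPlayers lookups.
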(event EventHandleStartingNewPlayer
  (params (NewPlayer :type Player%20Controller%20Object%20Reference))
  (|CallParentFunction NewPlayer)
  (CallFunction|AddPlayers NewPlayer))

(fn ConstructionScript)

(fn GetPlayers
  (params (IDPlayer :type Guid%20Structure%20%28by%20ref%29))
  (return (.Value (Utilities|Map|Find (Variables|Default|GetPlayers) IDPlayer))))

(fn AddPlayers
  (params (PC :type Player%20Controller%20Object%20Reference%20%28by%20ref%29))
  (bind _aspc_rts (Utilities|Casting|CastToPC_RTS PC))
  (bind (_idpc _name _color) (CallFunction|GenerateIDandData))
  (bind _dataplayer (Default|AssignIDandData _aspc_rts _idpc _name _color))
  (Utilities|Map|Add (Variables|Default|GetPlayers) _idpc PC)
  (Default|SetDataPlayer _aspc_rts _dataplayer))

(fn GenerateIDandData
  (return (Guid|NewGuid) (Utilities|String|StringToName (Utilities|String|ToString(Text) (Utilities|Text|FormatText "Fortea {x}" (Math|Random|RandomInteger 100)))) (Math|Color|MakeColor (Math|Random|RandomFloatinRange 0.0 1.0) (Math|Random|RandomFloatinRange 0.0 1.0) (Math|Random|RandomFloatinRange 0.0 1.0))))