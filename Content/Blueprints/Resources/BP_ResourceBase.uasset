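; Base Blueprint for selectable resource actors that supply their own info data and show a colored selection decal.
; On BeginPlay it caches its DT_ElementsUI row, looked up by IDUnit, and exposes it through GetInfo.
; Select adds a decal sized by CalculateScaleDecal, tints it through a dynamic material instance and returns that data.
; DeSelect destroys the decal component found by class.
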(event EventDeSelect
  (bind _returnvalue (Actor|GetComponentbyClass "/Script/Engine.DecalComponent"))
  (Utilities|IsValid _returnvalue
    (:Is%20Valid
      (Components|DestroyComponent _returnvalue))))

(event EventBeginPlay
  (bind _returnvalue (Utilities|GetDataTableRow "/Game/Blueprints/Structs/DT_ElementsUI.DT_ElementsUI" (Variables|Default|GetIDUnit))
    (:then
      (Variables|Default|SetData _returnvalue))))

(fn ConstructionScript)

(fn GetInfo
  (return (Variables|Default|GetData)))

(fn Select
  (params (Color :type Linear%20Color%20Structure))
  (bind _self self)
  (bind _scale (CallFunction|CalculateScaleDecal _self))
  (bind _returnvalue (AddComponent|AddDecalComponent false (Math|Transform|MakeTransform "0, 0, 0" "90.000000,0.000000,0.000000" (Math|Vector|MakeVector 1.0 (.y _scale) (.z _scale)))))
  (Rendering|Components|Decal|SetDecalMaterial _returnvalue "/Game/Materials/M_SelectedMaterial.M_SelectedMaterial")
  (bind _returnvalue_2 (Rendering|Material|CreateDynamicMaterialInstance "/Game/Materials/M_SelectedMaterial.M_SelectedMaterial" "None" "None" :!class /Script/Engine.KismetMaterialLibrary))
  (Rendering|Material|SetVectorParameterValue _returnvalue_2 "Color" Color :!class /Script/Engine.MaterialInstanceDynamic)
  (Rendering|Components|Decal|SetDecalMaterial _returnvalue _returnvalue_2)
  (return (CallFunction|GetInfo)))