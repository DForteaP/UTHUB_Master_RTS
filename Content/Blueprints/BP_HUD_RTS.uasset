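; RTS HUD Blueprint that creates the main W_Info interface at BeginPlay and pushes selected-item info and resource updates into it.
; Hovering Craft or Investigate actions opens the craft list for the selected item, with event delegates passed into the widgets.
; The Return function forwards craft data and the selected item to a cached PC_RTS to spawn craftables.
; A messages board is created on first use, binds a ping-type callback, then toggles visibility.
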(event EventBeginPlay
  (bind _returnvalue (UserInterface|CreateWidget "/Game/UI/W_Info.W_Info_C"))
  (bind _output_get (Variables|Default|SetMainUI _returnvalue))
  (UserInterface|Viewport|AddtoPlayerScreen _output_get))

(fn ConstructionScript)

(fn RefreshInfoItemSelected
  (params (Data :type S%20Data%20UI%20Structure) (ItemSelected :type Object%20Object%20Reference))
  (Variables|Default|SetItemSelected ItemSelected)
  (bind _output_get (Variables|Default|SetData Data))
  (Default|RefreshInfoUI (Variables|Default|GetMainUI) _output_get (EventDispatchers|CreateEvent :!event ShowHoverInfoAction) ItemSelected))

(fn ShowMessagesBoard
  (params (Event :type Delegate%20%28by%20ref%29))
  (Variables|Default|GetMessagesBoard
    (:then
      (if (Variables|Default|GetVisible?)
        (Widget|SetVisibility (Variables|Default|GetMessagesBoard) "Hidden")
        (Variables|Default|SetVisible? false)
        (else
          (Widget|SetVisibility (Variables|Default|GetMessagesBoard) "Visible")
          (Variables|Default|SetVisible? true))))
    (:else
      (bind _returnvalue (UserInterface|CreateWidget "/Game/UI/W_MessagesBoard.W_MessagesBoard_C"))
      (bind _output_get (Variables|Default|SetMessagesBoard _returnvalue))
      (UserInterface|Viewport|AddtoPlayerScreen _output_get)
      (EventDispatchers|BindEventtoReturnPingType _output_get Event)
      (Variables|Default|SetVisible? true))))

(fn RefreshInfoResorces
  (params (Resources :type Array%20of%20S%20Resource%20Amount%20Structures))
  (bind _mainui (Variables|Default|GetMainUI)
    (:then
      (Default|Refresh (Variables|/Game/UI/W_Info.W_Info_C|GetW_Resources _mainui) Resources))
    (:else)))

(fn GetPCRef
  (Variables|Default|GetPC%20RTS
    (:then
      _)
    (:else
      (bind _aspc_rts (Utilities|Casting|CastToPC_RTS (Game|Player|GetOwningPlayerController)))
      (Variables|Default|SetPC%20RTS _aspc_rts)))
  (return (Variables|Default|GetPC%20RTS)))

(fn ShowHoverInfoAction
  (params (Action :type E_Actions%20Enum :default "NewEnumerator0") (RowName :type Name))
  (switch Utilities|FlowControl|Switch|SwitchonE_Actions Action
    (:NewEnumerator3
      _)
    (:NewEnumerator10
      _))
  (CallFunction|ShowHover (EventDispatchers|CreateEvent :!event Return) RowName (Variables|Default|GetItemSelected)))

(fn ShowHover
  (params (Event :type Delegate%20%28by%20ref%29) (Name :type Name) (ItemSelected :type Object%20Object%20Reference))
  (bind _mainui (Variables|Default|GetMainUI))
  (bind _w_craftlist (Variables|/Game/UI/W_Info.W_Info_C|GetW_CraftList _mainui))
  (Widget|SetVisibility _w_craftlist "Visible")
  (Default|Init _w_craftlist Name Event ItemSelected))

(fn Return
  (params (Data :type S%20Crafteables%20Structure))
  (bind _itemselected (Variables|Default|GetItemSelected)
    (:then
      (Default|SpawnCrafteables (CallFunction|GetPCRef) Data _itemselected))
    (:else)))