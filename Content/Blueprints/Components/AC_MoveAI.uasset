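; AC_MoveAI is an AI order component that sends its AI controller to a target location.
; An order is valid only when the location is a valid AI location and the clicked actor carries the "floor" tag.
; Executing the action calls MoveToLocation on the base AI controller with the stored location.
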(event EventBeginPlay
  (|CallParentFunction) ; This node is disabled and will not be called.\nDrag off pins to build functionality.
)

(event EventTick
  (params (DeltaSeconds :type Float%20%28single-precision%29))
  (|CallParentFunction DeltaSeconds) ; This node is disabled and will not be called.\nDrag off pins to build functionality.
)

(fn IsValidforOrder
  (params (Location :type Vector :default "0, 0, 0") (Actor :type Actor%20Object%20Reference) (Id :type Name :default "None"))
  (return (and (AI|IsValidAILocation Location) (Actor|ActorHasTag Actor "floor"))))

(fn DoAction
  (AI|Navigation|MovetoLocation (Variables|Default|GetAIC%20Base) (Variables|Default|GetLocation) -1.0 true true false true 0))