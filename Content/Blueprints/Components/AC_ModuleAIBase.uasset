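; AC_ModuleAIBase is a base component for AI modules that are owned by an AIC_Base AI controller.
; It exposes IsValidForOrder, which takes a location, actor and id and returns false by default, and an empty DoAction, both apparently meant for child modules to override.
; GetAIController lazily casts the component's owner to AIC_Base and caches the reference for later calls.
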(event EventBeginPlay)

(event EventTick
  (params (DeltaSeconds :type Float%20%28single-precision%29)))

(fn IsValidforOrder
  (params (Location :type Vector) (Actor :type Actor%20Object%20Reference) (Id :type Name))
  (Variables|Default|SetLocation Location)
  (Variables|Default|SetActor Actor)
  (Variables|Default|SetId Id)
  (return false))

(fn DoAction)

(fn GetAIController
  (Variables|Default|GetAIC%20Base
    (:then
      _)
    (:else
      (bind _asaic_base (Utilities|Casting|CastToAIC_Base (Components|GetOwner)))
      (Variables|Default|SetAIC%20Base _asaic_base)))
  (return (Variables|Default|GetAIC%20Base)))